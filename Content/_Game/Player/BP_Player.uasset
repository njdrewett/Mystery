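; BP_Player is the player Blueprint that handles lock-on targeting and attack input.
; The lock-on input toggles the LockOnComponent with a fixed range, and that component's target-updated delegate passes the new target to the player's AnimInstance.
; The attack input prints a debug string and calls Attack on the CombatComponent.
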(event `EnhancedInput|/Game/_Game/Player/Control/Actions/IA_LockOn`
  (params (ActionValue :type Boolean) (ElapsedSeconds :type "Float (double-precision)") (TriggeredSeconds :type "Float (double-precision)") (InputAction :type "InputAction Object Reference" :default "/Game/_Game/Player/Control/Actions/IA_LockOn.IA_LockOn"))
  (:`Started`
    (`LockOnComponent.toggleLockOn` (`self.LockOnComponent`) 750.0)))

(event `self.LockOnComponent.OnUpdatedTargetDelegate`
  (params (newTargetActorRef :type "Actor Object Reference"))
  (`PlayerAnimInstance.updateLockOnTarget` (`self.playerAnimInstance`) newTargetActorRef))

(event `EnhancedInput|/Game/_Game/Player/Control/Actions/IA_Attack`
  (params (ActionValue :type Boolean) (ElapsedSeconds :type "Float (double-precision)") (TriggeredSeconds :type "Float (double-precision)") (InputAction :type "InputAction Object Reference" :default "/Game/_Game/Player/Control/Actions/IA_Attack.IA_Attack"))
  (:`Started`
    (`KismetSystemLibrary.PrintString` "Attack")
    (`CombatComponent.attack` (`self.CombatComponent`))))

(fn `UserConstructionScript`
  (`parent.UserConstructionScript`))